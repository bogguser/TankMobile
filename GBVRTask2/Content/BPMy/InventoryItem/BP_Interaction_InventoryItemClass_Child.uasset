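; Child of the interactive inventory item class that prototypes a timed explosive, using only debug prints.
; Its TriggerReleased event passes through a DoOnce into a DoN limited by the Tick variable.
; When the counter equals Tick it prints "BOOM"; otherwise it waits a second and prints the remaining count.
; No loop or DoOnce reset is wired, so the countdown advances only one step.
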(event EventBeginPlay
  (|CallParentFunction) ; This node is disabled and will not be called.\nDrag off pins to build functionality.
)

(event Collision|EventActorBeginOverlap
  (params (OtherActor :type Actor%20Object%20Reference))
  (|CallParentFunction OtherActor) ; This node is disabled and will not be called.\nDrag off pins to build functionality.
)

(event EventTick
  (params (DeltaSeconds :type Float%20%28single-precision%29))
  (|CallParentFunction DeltaSeconds) ; This node is disabled and will not be called.\nDrag off pins to build functionality.
)

(event EventTriggerReleased
  (Utilities|FlowControl|DoOnce false
    (:Completed
      (bind _counter (Utilities|FlowControl|DoN (Variables|Default|GetTick))
        (:Exit
          (if (== (Variables|Default|GetTick) _counter)
            (Development|PrintString "BOOM")
            (else
              (Utilities|FlowControl|Delay 1.0)
              (Development|PrintString (Utilities|String|ToString(Integer) (- (Variables|Default|GetTick) _counter)) true true "(R=0.000000,G=0.660000,B=1.000000,A=1.000000)" 5.0))))))))

(fn ConstructionScript
  (|CallParentFunction))