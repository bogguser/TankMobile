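; BP_interactableDoors is a double sliding door actor in the quest system demo that opens or closes when interacted with.
; Each Interact event toggles a FlipFlop that moves two cube components in opposite directions between two relative positions over a timed MoveComponentTo.
; Both moves feed OnInteractionFinished with the interacting actor, so it is called for each panel's move.
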(event EventBeginPlay)

(event Collision|EventActorBeginOverlap
  (params (OtherActor :type Actor%20Object%20Reference)))

(event EventTick
  (params (DeltaSeconds :type Float%20%28single-precision%29)))

(event EventInteract
  (params (ActorInteractionWithObject :type Actor%20Object%20Reference))
  (Utilities|FlowControl|FlipFlop
    (:A
      (Utilities|FlowControl|Sequence
        (:then_0
          (Components|MoveComponentTo (Variables|Default|GetCube) "-4000.000000, 0, 0" "0, 0, 0" false false 1.0 false))
        (:then_1
          (Components|MoveComponentTo (Variables|Default|GetCube1) "4000.000000, 0, 0" "0, 0, 0" false false 1.0 false))))
    (:B
      (Utilities|FlowControl|Sequence
        (:then_0
          (Components|MoveComponentTo (Variables|Default|GetCube) "-2000.000000, 0, 0" "0, 0, 0" false false 1.0 false))
        (:then_1
          (Components|MoveComponentTo (Variables|Default|GetCube1) "2000.000000, 0, 0" "0, 0, 0" false false 1.0 false)))))
  (Class|InteractableActor|OnInteractionFinished ActorInteractionWithObject))

(fn ConstructionScript)