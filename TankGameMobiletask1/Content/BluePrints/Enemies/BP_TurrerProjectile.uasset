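; BP_TurrerProjectile is an enemy Blueprint with a health component and an enemy health bar widget.
; Tick fetches and casts the HealHud widget every frame, caches it, and sets its progress bar from current over max health.
; The Hit event plays the bar's hit animation while health remains above zero.
; The graph holds no movement, damage or death logic.
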(event EventBeginPlay)

(event Collision|EventActorBeginOverlap
  (params (OtherActor :type Actor%20Object%20Reference)))

(event Collision|EventHit
  (params (MyComp :type Primitive%20Component%20Object%20Reference) (Other :type Actor%20Object%20Reference) (OtherComp :type Primitive%20Component%20Object%20Reference) (bSelfMoved :type Boolean) (HitLocation :type Vector :default "0, 0, 0") (HitNormal :type Vector :default "0, 0, 0") (NormalImpulse :type Vector :default "0, 0, 0") (Hit :type Hit%20Result%20Structure%20%28by%20ref%29))
  ;[1 1 1] HealBar
  (if (> (Variables|/Script/TankGame.HealthComponent|GetCurretHealth (Variables|Default|GetHealthComponent)) 0.0)
    (UserInterface|Animation|PlayAnimation (stale EventTick _aswbp_health_bar_enemy) (Variables|/Game/BluePrints/WBP/WBP_HealthBarEnemy.WBP_HealthBarEnemy_C|GetAnimationHit (stale EventTick _aswbp_health_bar_enemy)) 0.0 1 "Forward" 1.0 false)))

(event EventTick
  (params (DeltaSeconds :type Float%20%28single-precision%29))
  (bind _healthcomponent (Variables|Default|GetHealthComponent))
  ;[1 1 1] HealBar
  (bind _aswbp_health_bar_enemy (Utilities|Casting|CastToWBP_HealthBarEnemy (UserInterface|GetUserWidgetObject (Variables|Default|GetHealHud))))
  (Progress|SetPercent (Variables|/Game/BluePrints/WBP/WBP_HealthBarEnemy.WBP_HealthBarEnemy_C|GetProgressBar_0 _aswbp_health_bar_enemy) (/ (Variables|/Script/TankGame.HealthComponent|GetCurretHealth _healthcomponent) (Variables|/Script/TankGame.HealthComponent|GetMaxHealth _healthcomponent))))

(fn ConstructionScript)