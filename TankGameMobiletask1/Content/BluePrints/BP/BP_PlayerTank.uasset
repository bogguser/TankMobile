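; Player tank Blueprint that acts as the hub for the player's UI and forwards the Interact input to its Interaction component.
; BeginPlay adds mobile controls, map and HUD, whose health bar refreshes from HealthComponent on Hit.
; Input events open save, quest log, media, map, pause, tank and turret widgets, several toggled by FlipFlop, with pause and tank screens pausing the game.
; Destruction shows the game-over widget with UI-only input.
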(event EventBeginPlay
  (bind _returnvalue (Game|GetPlayerController 0))
  (bind _healthcomponent (Variables|Default|GetHealthComponent))
  (Utilities|FlowControl|Sequence
    (:then_0
      (bind _returnvalue_2 (UserInterface|CreateWidget "/Game/BluePrints/WBP/WBP_ConrollerMobile.WBP_ConrollerMobile_C" _returnvalue))
      (UserInterface|Viewport|AddtoViewport _returnvalue_2 0))
    (:then_1
      ;[1 1 1] Maps
      (bind _returnvalue_3 (UserInterface|CreateWidget "/Game/BluePrints/MiniMaps/WBP_Maps.WBP_Maps_C" (Game|GetPlayerController 0)))
      (bind _output_get (Variables|Default|SetMap _returnvalue_3))
      (UserInterface|Viewport|AddtoViewport _output_get 1)
      ;[1 1 1] Update and create widget health bar
      (bind _returnvalue_4 (UserInterface|CreateWidget "/Game/BluePrints/WBP/WBP_PlayerHUD.WBP_PlayerHUD_C" _returnvalue))
      (bind _output_get_2 (Variables|Default|SetHudReference _returnvalue_4))
      (UserInterface|Viewport|AddtoViewport _output_get_2 1)
      (Default|UpdateHealth (Variables|Default|GetHudReference) (Variables|/Script/TankGame.HealthComponent|GetCurretHealth _healthcomponent) (Variables|/Script/TankGame.HealthComponent|GetMaxHealth _healthcomponent)))))

(event Collision|EventActorBeginOverlap
  (params (OtherActor :type Actor%20Object%20Reference)))

(event EventTick
  (params (DeltaSeconds :type Float%20%28single-precision%29)))

(event EventDestroyed
  ;[1 1 1] Create Widget GameOver
  (bind _returnvalue (UserInterface|CreateWidget "/Game/BluePrints/WBP/WBP_GameOver.WBP_GameOver_C"))
  (UserInterface|Viewport|AddtoViewport _returnvalue 0)
  (Input|SetInputModeUIOnly (Game|GetPlayerController 0) _returnvalue "LockAlways"))

(event Collision|EventHit
  (params (MyComp :type Primitive%20Component%20Object%20Reference) (Other :type Actor%20Object%20Reference) (OtherComp :type Primitive%20Component%20Object%20Reference) (bSelfMoved :type Boolean) (HitLocation :type Vector :default "0, 0, 0") (HitNormal :type Vector :default "0, 0, 0") (NormalImpulse :type Vector :default "0, 0, 0") (Hit :type Hit%20Result%20Structure%20%28by%20ref%29))
  (bind _healthcomponent (Variables|Default|GetHealthComponent))
  ;[1 1 1] Update and create widget health bar
  (Default|UpdateHealth (Variables|Default|GetHudReference) (Variables|/Script/TankGame.HealthComponent|GetCurretHealth _healthcomponent) (Variables|/Script/TankGame.HealthComponent|GetMaxHealth _healthcomponent)))

(event Input|ActionEvents|InputActionInteract
  (params (Key :type Key%20Structure :default "None"))
  ;[1 1 1] Interact
  (:Pressed
    (Class|InteractionComponent|Interact (Variables|Default|GetInteraction))))

(event Input|ActionEvents|InputActionQuestLog
  (params (Key :type Key%20Structure :default "None"))
  (bind _returnvalue (Game|GetPlayerController 0))
  ;[1 1 1] QuestLog
  (:Pressed
    (Utilities|FlowControl|FlipFlop
      (:A
        (bind _returnvalue_2 (UserInterface|CreateWidget "/QuestSystem/Widgets/W_QuestLog.W_QuestLog_C" _returnvalue))
        (Class|QuestLogWidget|Init _returnvalue_2 (Variables|Default|GetQuestListComponent))
        (UserInterface|Viewport|AddtoViewport _returnvalue_2 0)
        (Input|SetInputModeGameandUI _returnvalue _returnvalue_2 "DoNotLock" true)
        (Variables|/Script/Engine.PlayerController|SetbShowMouseCursor _returnvalue true))
      (:B
        (Widget|RemovefromParent _returnvalue_2)
        (Input|SetInputModeGameOnly _returnvalue)
        (Variables|/Script/Engine.PlayerController|SetbShowMouseCursor _returnvalue false)))))

(event Input|KeyboardEvents|P
  (params (Key :type Key%20Structure :default "None"))
  ;[1 1 1] Maps
  (:Pressed
    (Utilities|FlowControl|FlipFlop
      (:A
        (bind _returnvalue (UserInterface|CreateWidget "/Game/BluePrints/MiniMaps/WBP_MiniMapsMenu.WBP_MiniMapsMenu_C" (Game|GetPlayerController 0)))
        (bind _output_get (Variables|Default|SetMapMenu _returnvalue))
        (UserInterface|Viewport|AddtoViewport _output_get 1))
      (:B
        (Widget|RemovefromParent _output_get)))))

(event Input|KeyboardEvents|M
  (params (Key :type Key%20Structure :default "None"))
  (bind _returnvalue (Game|GetPlayerController 0))
  ;[1 1 1] Widget Pause
  (:Pressed
    (Variables|/Script/Engine.PlayerController|SetbShowMouseCursor _returnvalue true)
    (Game|SetGamePaused true)
    (bind _returnvalue_2 (UserInterface|CreateWidget "/Game/BluePrints/WBP/WBP_PauseMenu.WBP_PauseMenu_C"))
    (UserInterface|Viewport|AddtoViewport _returnvalue_2 0)
    (Input|SetInputModeUIOnly _returnvalue _returnvalue_2 "LockAlways")))

(event Input|KeyboardEvents|Y
  (params (Key :type Key%20Structure :default "None"))
  (bind _returnvalue (Game|GetPlayerController 0))
  ;[1 1 1] SpawnedTurret
  (:Pressed
    (Variables|/Script/Engine.PlayerController|SetbShowMouseCursor _returnvalue true)
    (bind _returnvalue_2 (UserInterface|CreateWidget "/Game/BluePrints/WBP/WBP_Turrets.WBP_Turrets_C" _returnvalue))
    (UserInterface|Viewport|AddtoViewport _returnvalue_2 1)
    (Input|SetInputModeGameandUI _returnvalue _returnvalue_2 "DoNotLock" true)))

(event Input|KeyboardEvents|O
  (params (Key :type Key%20Structure :default "None"))
  (bind _returnvalue (Game|GetPlayerController 0))
  ;[1 1 1] SaveGame
  (:Pressed
    (Variables|/Script/Engine.PlayerController|SetbShowMouseCursor _returnvalue true)
    (Utilities|FlowControl|FlipFlop
      (:A
        (bind _returnvalue_2 (UserInterface|CreateWidget "/Game/Widgets/W_TankSaveGame.W_TankSaveGame_C" _returnvalue))
        (UserInterface|Viewport|AddtoViewport _returnvalue_2 1))
      (:B
        (Variables|/Script/Engine.PlayerController|SetbShowMouseCursor _returnvalue false)
        (Widget|RemovefromParent _returnvalue_2)))))

(event Input|KeyboardEvents|J
  (params (Key :type Key%20Structure :default "None"))
  (bind _returnvalue (Game|GetPlayerController 0))
  ;[1 1 1] MediaPlayer
  (:Pressed
    (Variables|/Script/Engine.PlayerController|SetbShowMouseCursor _returnvalue true)
    (Utilities|FlowControl|FlipFlop
      (:A
        (bind _returnvalue_2 (UserInterface|CreateWidget "/MediaWidget/WBP_MediaWidget.WBP_MediaWidget_C" _returnvalue))
        (bind _output_get (Variables|Default|SetNewVar_1 _returnvalue_2))
        (UserInterface|Viewport|AddtoViewport _output_get 1))
      (:B
        (Widget|RemovefromParent _output_get)))))

(event Input|KeyboardEvents|H
  (params (Key :type Key%20Structure :default "None"))
  (bind _returnvalue (Game|GetPlayerController 0))
  ;[1 1 1] DraggableText
  (:Pressed
    (Variables|/Script/Engine.PlayerController|SetbShowMouseCursor _returnvalue true)
    (Game|SetGamePaused true)
    (bind _returnvalue_2 (UserInterface|CreateWidget "/Game/BluePrints/WBP/WBP_Tanks.WBP_Tanks_C" _returnvalue))
    (UserInterface|Viewport|AddtoViewport _returnvalue_2 1)
    (Input|SetInputModeUIOnly _returnvalue _returnvalue_2 "LockAlways")))

(fn ConstructionScript)