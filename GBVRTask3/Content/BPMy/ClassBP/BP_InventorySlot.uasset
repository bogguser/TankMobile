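; BP_InventorySlot is an inventory slot actor for motion-controller interaction that tracks the item resting in it.
; Sphere overlap events store an entering BP_Interaction_InventoryItemClass as ItemInSlot and clear it when that same item leaves.
; The Put event calls TryGrab on the stored item's GrabComponent with MotionController, then moves the item to the slot's location, without checking that an item is set.
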(event OnComponentBeginOverlap(Sphere)
  (params (OverlappedComponent :type Primitive%20Component%20Object%20Reference) (OtherActor :type Actor%20Object%20Reference) (OtherComp :type Primitive%20Component%20Object%20Reference) (OtherBodyIndex :type Integer) (bFromSweep :type Boolean) (SweepResult :type Hit%20Result%20Structure%20%28by%20ref%29))
  (bind _asbp_interaction_inventory_item_class (Utilities|Casting|CastToBP_Interaction_InventoryItemClass OtherActor))
  (Variables|Default|SetItemInSlot _asbp_interaction_inventory_item_class))

(event OnComponentEndOverlap(Sphere)
  (params (OverlappedComponent :type Primitive%20Component%20Object%20Reference) (OtherActor :type Actor%20Object%20Reference) (OtherComp :type Primitive%20Component%20Object%20Reference) (OtherBodyIndex :type Integer))
  (bind _asbp_interaction_inventory_item_class (Utilities|Casting|CastToBP_Interaction_InventoryItemClass OtherActor))
  (if (== _asbp_interaction_inventory_item_class (Variables|Default|GetItemInSlot))
    (Variables|Default|SetItemInSlot 0)))

(event Custom|Put
  (Default|TryGrab (Variables|/Game/BPMy/ClassBP/BP_Interaction_Class.BP_Interaction_Class_C|GetGrabComponent (Variables|Default|GetItemInSlot)) (Variables|Default|GetMotionController))
  (Transformation|SetActorLocation (Variables|Default|GetItemInSlot) (Transformation|GetActorLocation) false false))

(event EventBeginPlay)

(event Collision|EventActorBeginOverlap
  (params (OtherActor :type Actor%20Object%20Reference)))

(event EventTick
  (params (DeltaSeconds :type Float%20%28single-precision%29)))

(fn ConstructionScript)