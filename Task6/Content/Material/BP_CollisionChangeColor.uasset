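; Collision-trigger actor that recolors a BP_ChangeColor actor when something begins overlapping its R component.
; On overlap it takes the first BP_ChangeColor found in the level and creates a dynamic material instance on its Sphere from the current material.
; It sets the instance's color parameter to green and applies it to that actor's static mesh.
; Nothing restores the original material; the node storing it is unconnected.
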(event OnComponentBeginOverlap(r)
  (params (OverlappedComponent :type Primitive%20Component%20Object%20Reference) (OtherActor :type Actor%20Object%20Reference) (OtherComp :type Primitive%20Component%20Object%20Reference) (OtherBodyIndex :type Integer) (bFromSweep :type Boolean) (SweepResult :type Hit%20Result%20Structure%20%28by%20ref%29))
  (bind _outactors (Actor|GetAllActorsOfClass "/Game/Material/BP_ChangeColor.BP_ChangeColor_C"))
  (bind _output_get (Variables|Default|SetInteractiveActor (Utilities|Array|Get(acopy) _outactors)))
  (bind _interactiveactor (Variables|Default|GetInteractiveActor)
    (:then
      (bind _returnvalue (Rendering|Material|CreateDynamicMaterialInstance (Variables|/Game/Material/BP_ChangeColor.BP_ChangeColor_C|GetSphere _interactiveactor) 0 (Rendering|Material|GetMaterial (Actor|GetComponentbyClass _output_get "/Script/Engine.StaticMeshComponent") 0) "" :!class /Script/Engine.PrimitiveComponent))
      (bind _output_get_2 (Variables|Default|SetInstance _returnvalue))
      (Rendering|Material|SetVectorParameterValue _output_get_2 "Color Param" "(R=0.108706,G=0.500000,B=0.000000,A=1.000000)" :!class /Script/Engine.MaterialInstanceDynamic)
      (Rendering|Material|SetMaterial (Actor|GetComponentbyClass _output_get "/Script/Engine.StaticMeshComponent") 0 _output_get_2))
    (:else)))

(event EventBeginPlay)

(event Collision|EventActorBeginOverlap
  (params (OtherActor :type Actor%20Object%20Reference)))

(event EventTick
  (params (DeltaSeconds :type Float%20%28single-precision%29)))

(fn ConstructionScript)