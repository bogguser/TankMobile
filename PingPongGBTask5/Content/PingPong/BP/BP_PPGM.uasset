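; BP_PPGM, apparently the PingPong game mode, holds the match start until both players are present, then spawns the ball.
; On BeginPlay it shows a waiting widget and starts a looping timer that polls whether Player1Start and Player2Start are valid.
; Once both are, it clears that timer and, after a short delay, spawns BP_Ball at Player2Start and removes the widget.
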(event Custom|CheckTwoPlayer
  (if (and (Utilities|IsValid (Variables|Default|GetPlayer1Start)) (Utilities|IsValid (Variables|Default|GetPlayer2Start)))
    (Utilities|Time|SetTimerbyEvent (delegate Custom|SpawnBallEvent) 2.0)
    (Utilities|Time|ClearandInvalidateTimerbyHandle (Variables|Default|GetNewVar_0))))

(event Custom|SpawnBallEvent
  (Game|SpawnActorfromClass "/Game/PingPong/BP/BP_Ball.BP_Ball_C" (Transformation|GetActorTransform (Variables|Default|GetPlayer2Start)) "AdjustIfPossibleButAlwaysSpawn" 0 0)
  (Widget|RemovefromParent (stale EventBeginPlay _returnvalue_2)))

(event EventBeginPlay
  (bind _returnvalue (Utilities|Time|SetTimerbyEvent (delegate Custom|CheckTwoPlayer) 1.0 true))
  (Variables|Default|SetNewVar_0 _returnvalue)
  (bind _returnvalue_2 (UserInterface|CreateWidget "/Game/PingPong/BP/WBP_WaitPlayer.WBP_WaitPlayer_C" (Game|GetPlayerController 0)))
  (UserInterface|Viewport|AddtoViewport _returnvalue_2 0))

(event EventTick
  (params (DeltaSeconds :type Float%20%28single-precision%29)))

(fn ConstructionScript)