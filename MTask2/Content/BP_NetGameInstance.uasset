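; Game instance that hosts and joins multiplayer sessions and reports network and travel errors.
; CreateGame creates a LAN session, then opens ThirdPersonExampleMap as a listen server or prints a creation error.
; JoinSessionInstance joins a supplied search result for the first player controller, with no success or failure handling.
; The network and travel error handlers print the failure type on screen.
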(event Custom|JoinSessionInstance
  (params (SearchResult :type Blueprint%20Session%20Result%20Structure%20%28by%20ref%29))
  (|JoinSession (Game|GetPlayerController 0) SearchResult))

(event Custom|CreateGame
  (|Session (Game|GetPlayerController 0) 16 true
    (:OnSuccess
      (Game|OpenLevel(byName) "ThirdPersonExampleMap" true "listen"))
    (:OnFailure
      (Development|PrintString "Creation error"))))

(event EventHandleNetworkError
  (params (FailureType :type ENetworkFailure%20Enum :default "NetDriverAlreadyExists") (bIsServer :type Boolean))
  (Development|PrintString (Utilities|String|EnumtoString FailureType)))

(event EventHandleTravelError
  (params (FailureType :type ETravelFailure%20Enum :default "NoLevel"))
  (Development|PrintString (Utilities|String|EnumtoString FailureType)))