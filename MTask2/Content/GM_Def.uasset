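; GM_Def is a game mode that balances joining players between two teams.
; On PostLogin it puts each BP_PlayerController on Team 2 if Team 1 is larger, otherwise Team 1, setting its TeamID and printing debug text.
; On logout it removes the last array entry rather than the leaving controller, and checks Team 2 against ID 0 although it assigns 2, so Team 2 departures are missed.
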(event EventBeginPlay)

(event EventTick
  (params (DeltaSeconds :type Float%20%28single-precision%29)))

(event EventPostLogin
  (params (NewPlayer :type Player%20Controller%20Object%20Reference))
  (bind _team2 (Variables|Default|GetTeam2))
  (bind _team1 (Variables|Default|GetTeam1))
  (bind _asbp_player_controller (Utilities|Casting|CastToBP_PlayerController NewPlayer)
    (:then
      (if (> (Utilities|Array|Length _team1) (Utilities|Array|Length _team2))
        (Default|SetTeamID _asbp_player_controller 2)
        (Utilities|Array|Add _team2 _asbp_player_controller)
        (Development|PrintString "2")
        (else
          (Default|SetTeamID _asbp_player_controller 1)
          (Utilities|Array|Add _team1 _asbp_player_controller)
          (Development|PrintString "1"))))
    (:CastFailed
      (Development|PrintString "POSTLOGINERROR 
"))))

(event EventOnLogout
  (params (ExitingController :type Controller%20Object%20Reference))
  (bind _team1 (Variables|Default|GetTeam1))
  (bind _team2 (Variables|Default|GetTeam2))
  (bind _asbp_player_controller (Utilities|Casting|CastToBP_PlayerController ExitingController))
  (if (== (Variables|/Game/ThirdPersonCPP/Blueprints/BP_PlayerController.BP_PlayerController_C|GetTeamID _asbp_player_controller) 1)
    (Utilities|Array|RemoveIndex _team1 (Utilities|Array|LastIndex _team1))
    (elif (== (Variables|/Game/ThirdPersonCPP/Blueprints/BP_PlayerController.BP_PlayerController_C|GetTeamID _asbp_player_controller) 0)
      (Utilities|Array|RemoveIndex _team2 (Utilities|Array|LastIndex _team2)))))

(fn ConstructionScript)